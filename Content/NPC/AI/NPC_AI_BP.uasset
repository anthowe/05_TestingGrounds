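; NPC AI controller that runs the Patrol behavior tree for its pawn.
; On BeginPlay it sets up the PatrolData blackboard, stores the blackboard component in a variable and starts the tree.
; AI Perception target updates only print a debug string naming the controlled pawn, the sense class and the detected actor, without feeding the blackboard.
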(event `self.ReceiveBeginPlay`
  (bind _blackboardcomponent (`self.UseBlackboard` "/Game/NPC/AI/PatrolData.PatrolData"))
  (set `self.NewVar_0` _blackboardcomponent)
  (`self.RunBehaviorTree` "/Game/NPC/AI/Patrol.Patrol"))

(event `self.AIPerception.OnTargetPerceptionUpdated`
  (params (Actor :type "Actor Object Reference") (Stimulus :type "AIStimulus Structure"))
  (bind _returnvalue (`AIPerceptionSystem.GetSenseClassForStimulus` Stimulus))
  (`KismetSystemLibrary.PrintString` (`KismetStringLibrary.Concat_StrStr` (`KismetSystemLibrary.GetObjectName` (`self.K2_GetPawn`)) "     " (`KismetSystemLibrary.GetClassDisplayName` _returnvalue) "     " (`KismetSystemLibrary.GetObjectName` Actor)) true true (struct :`G` 0.66 :`B` 1.0 :`A` 1.0) 20.0))

(fn `UserConstructionScript`)